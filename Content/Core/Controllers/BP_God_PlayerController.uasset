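; Player controller for the God character, forwarding camera look input and handling zoom on the controlled pawn.
; It caches the pawn as BP_GodCharacter on BeginPlay, and Check My Pawn re-casts and refreshes that reference whenever it is invalid.
; Look axes call the pawn's LookUp and LookRight.
; Zoom In plays or reverses a timeline that incrementally lowers or raises the first-person camera's field of view by the curve value each update.
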(event `self.ReceiveBeginPlay`
  ;[1 1 1] Get controlled pawn and cast it to God class
  (bind _asbp_god_character (cast `/Game/Core/Characters/BP_GodCharacter` (`self.K2_GetPawn`)))
  (set `self.My Pawn` _asbp_god_character))

(event `InputAxis|Look Up`
  (params (AxisValue :type "Float (single-precision)"))
  ;[1 1 1] Camera control
  (bind _my_pawn (`self.Check My Pawn`))
  (`/Game/Core/Characters/BP_GodCharacter.Look Up` _my_pawn AxisValue))

(event `InputAxis|Look Right`
  (params (AxisValue :type "Float (single-precision)"))
  ;[1 1 1] Camera control
  (bind _my_pawn (`self.Check My Pawn`))
  (`/Game/Core/Characters/BP_GodCharacter.Look Right` _my_pawn AxisValue))

(event `InputAction|Zoom In`
  (params (Key :type "Key Structure"))
  (bind _firstpersoncamera (`/Game/Core/Characters/BP_GodCharacter.FirstPersonCamera` (`self.My Pawn`)))
  (bind _fieldofview (`CameraComponent.FieldOfView` _firstpersoncamera))
  ;[1 1 1] Camera control
  (:`Pressed`
    (`self.Check My Pawn`)
    (bind (_direction _value) (`Timeline|Camera Zoom` :`NewTime` 0.0 :!label _label)
      (:`Update`
        (if (`|EnumEquality` _direction "Forward")
          (`CameraComponent.SetFieldOfView` _firstpersoncamera (- _fieldofview _value))
          (else
            (`CameraComponent.SetFieldOfView` _firstpersoncamera (+ _fieldofview _value)))))))
  (:`Released`
    (`self.Check My Pawn`)
    (goto _label :!via `Reverse`)))

(fn `UserConstructionScript`)